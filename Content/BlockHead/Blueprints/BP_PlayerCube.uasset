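; BP_PlayerCube is the player's cube, which propels itself forward along X.
; Each Tick applies an impulse to the PlayerCube component, scaling ForwardForce by DeltaSeconds for framerate independence.
; Disconnected logic remains for a jump impulse and for toggling the first PointLight found in the level, but neither runs.
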(event EventBeginPlay)

(event EventTick
  (params (DeltaSeconds :type Float%20%28single-precision%29))
  ;[0.175 1 0.3813] Player Character Moves Forward Using a Constant Framerate Indendent Impulse Force
  (bind _output_get (Variables|Default|SetDeltaSeconds DeltaSeconds))
  (Physics|AddImpulse (Variables|Default|GetPlayerCube) (Math|Vector|MakeVector (* _output_get (Variables|Default|GetForwardForce)) 0.0 0.0) "None" false))

(event Input|ActionEvents|InputActionToggleLights
  (params (Key :type Key%20Structure :default "None"))
  ;[1 0.2999 0.8461] Allow The User To Toggle The Pink Point Light On and Off Using the ToggleLights Action Mapping
)

(event Input|ActionEvents|InputActionJump
  (params (Key :type Key%20Structure :default "None"))
  ;[1 0.2999 0.8461] Jump Functionality (Disabled Until Needed in Gameplay)
)

(fn ConstructionScript)