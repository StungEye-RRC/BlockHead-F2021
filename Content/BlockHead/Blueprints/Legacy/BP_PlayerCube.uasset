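; BP_PlayerCube is the player's physics cube, pushed forward by a constant force and steered sideways by axis input.
; Hitting a BP_Obstacle or falling below a kill Z calls PlayerDied, while overlapping BP_EndPoint completes the level, both reported to BP_GameMode.
; A LevelEnded flag blocks steering and zeroes velocity each tick, preventing accidental wins on leftover momentum.
; Jump and light-toggle logic are present but unconnected.
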(event OnComponentHit(PlayerCube)
  (params (HitComponent :type Primitive%20Component%20Object%20Reference) (OtherActor :type Actor%20Object%20Reference) (OtherComp :type Primitive%20Component%20Object%20Reference) (NormalImpulse :type Vector :default "0, 0, 0") (Hit :type Hit%20Result%20Structure%20%28by%20ref%29))
  ;[0.175 1 0.3813] Call Player Died Function When Player Character Hits an Obstacle
  (Utilities|Casting|CastToBP_Obstacle OtherActor)
  (CallFunction|PlayerDied))

(event OnComponentBeginOverlap(PlayerCube)
  (params (OverlappedComponent :type Primitive%20Component%20Object%20Reference) (OtherActor :type Actor%20Object%20Reference) (OtherComp :type Primitive%20Component%20Object%20Reference) (OtherBodyIndex :type Integer) (bFromSweep :type Boolean) (SweepResult :type Hit%20Result%20Structure%20%28by%20ref%29))
  ;[0.175 1 0.3813] When Player Overlaps BP_EndPoint Set Level Ended Boolean and Tell GameMode that Level is Complete
  (Utilities|Casting|CastToBP_EndPoint OtherActor)
  (Variables|Default|SetbLevelEnded true)
  (Default|LevelComplete (Variables|Default|GetBP%20Game%20Mode)))

(event EventBeginPlay
  ;[0.114 0.9702 1] Get a Reference to BP_GameMode on Begin Play
  (bind _asbp_game_mode (Utilities|Casting|CastToBP_GameMode (Game|GetGameMode)))
  (Variables|Default|SetBP%20Game%20Mode _asbp_game_mode))

(event EventTick
  (params (DeltaSeconds :type Float%20%28single-precision%29))
  ;[0.114 0.9702 1] Player Character Moves Forward Using a Constant Framerate Indendent Force
  (if (Variables|Default|GetbLevelEnded)
    ;[0.175 1 0.3813] Stop All Motion When Level Ends. Prevents Accidental Wins on Final Momentum after touching an obstacle
    (Physics|SetPhysicsLinearVelocity (Variables|Default|GetPlayerCube) "0, 0, 0" false "None")
    (else
      (Physics|AddForce (Variables|Default|GetPlayerCube) (Math|Vector|MakeVector (Variables|Default|GetForwardForce) 0.0 0.0) "None" false)
      ;[0.175 1 0.3813] Player Loses If They Fall Off the Edge
      (if (< (.z (Transformation|GetActorLocation)) (Variables|Default|GetPlayerKillZ))
        (CallFunction|PlayerDied)))))

(event Input|ActionEvents|InputActionToggleLights
  (params (Key :type Key%20Structure :default "None"))
  ;[1 0.2999 0.8461] Allow The User To Toggle The Pink Point Light On and Off Using the ToggleLights Action Mapping
)

(event Input|ActionEvents|InputActionJump
  (params (Key :type Key%20Structure :default "None"))
  ;[1 0.2999 0.8461] Jump Functionality (Disabled Until Needed in Gameplay)
)

(event Input|AxisEvents|InputAxisMoveLeftRight
  (params (AxisValue :type Float%20%28single-precision%29))
  ;[0.114 0.9702 1] User Control Of Side to Side Movement Using a Force
  (if (not (Variables|Default|GetbLevelEnded))
    (Physics|AddForce (Variables|Default|GetPlayerCube) (Math|Vector|MakeVector 0.0 (* AxisValue (Variables|Default|GetSidewayForce)) 0.0) "None" false)))

(fn ConstructionScript)

(fn PlayerDied
  ;[0.175 1 0.3813] When Player Dies Set the Level Ended Boolean to True
  (if (not (Variables|Default|GetbLevelEnded))
    (Variables|Default|SetbLevelEnded true)
    (Default|EndGame (Variables|Default|GetBP%20Game%20Mode))))